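; HexGrid1_Blueprint generates a centred hexagonal grid of XSize by YSize cells in its construction script.
; It clears existing hexagons, then loops over columns and rows, adding a Default-type hexagon at each computed transform on a flat Z plane.
; Columns sit three-quarters of XScale apart, with odd ones shifted half a YScale to interlock.
; The event graph contains only empty event stubs.
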(event EventBeginPlay)

(event EventActorBeginOverlap
  (params (OtherActor :type Actor%20Object%20Reference)))

(event EventTick
  (params (DeltaSeconds :type Float%20%28single-precision%29)))

(fn ConstructionScript
  (bind _y_scale (LocalVariables|GetY%20Scale))
  (bind _x_size (Variables|Default|GetX%20Size))
  (bind _y_size (Variables|Default|GetY%20Size))
  (Class|HexGrid|ClearHexagons)
  (for _index (range 0 (- _x_size 1))
    (for _index_2 (range 0 (- _y_size 1))
      (Class|HexGrid|AddHexagon (Utilities|Struct|MakeHexagon (Math|Transform|MakeTransform (Math|Vector|MakeVector (* (- (Math|Conversions|ToFloat(Integer) _index) (* _x_size 0.5)) (* (LocalVariables|GetX%20Scale) 0.75)) (+ (* (Math|Integer|%(Integer) _index 2) (* _y_scale 0.5)) (* (- (Math|Conversions|ToFloat(Integer) _index_2) (* _y_size 0.5)) _y_scale)) 0.0)) "HE_Default")))))