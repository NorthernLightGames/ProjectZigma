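; Hex grid chunk Blueprint that generates a rectangular block of hexagon cells.
; The construction script loops over rows and columns centered on zero, using half of Height and Width as bounds, and adds a Default-type hexagon at each X/Y coordinate.
; It then passes the array to SetHexagons.
; The event graph holds only empty event stubs, so it adds no runtime logic.
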(event EventBeginPlay)

(event EventActorBeginOverlap
  (params (OtherActor :type Actor%20Object%20Reference)))

(event EventTick
  (params (DeltaSeconds :type Float%20%28single-precision%29)))

(fn ConstructionScript
  (bind _height (Variables|Default|GetHeight))
  (bind _width (Variables|Default|GetWidth))
  (bind _hexagons (LocalVariables|GetHexagons))
  (bind _returnvalue (/ _width 2))
  (bind _returnvalue_2 (/ _height 2))
  (for _index (range (* _returnvalue_2 -1) _returnvalue_2)
    (for _index_2 (range (* _returnvalue -1) _returnvalue)
      (Utilities|Array|Add _hexagons (Utilities|Struct|MakeHexagon _index_2 _index "HE_Default"))))
  (Class|Hexagons|SetHexagons _hexagons))